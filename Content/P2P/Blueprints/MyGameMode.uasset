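; Game mode for a P2P game that handles server-side respawning and HUD setup after login.
; RespawnRunOnServer spawns an actor at the first PlayerStart found, has the player's controller possess it, then destroys the old pawn.
; PostLogin creates the HUD for a local controller after a short Delay, since the player character may not exist yet, and calls ClientPostLogin on remote controllers.
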(event `Respawn RunOnServer`
  (params (Player :type "PlayerController Object Reference") (Pawn :type "Pawn Object Reference"))
  ;[1 1 1] リスポーン処理の本体 ※リスポーンは必ずサーバーで行うためにここを呼ぶ必要がある。
  (bind _outactors (`GameplayStatics.GetAllActorsOfClass` "/Script/Engine.PlayerStart"))
  (for _array_element _outactors
    (bind _returnvalue (`|SpawnActorFromClass` null (`self.GetTransform` _array_element) "Undefined" "OverrideRootScale" Player))
    (`Controller.Possess` Player _returnvalue)
    (`self.K2_DestroyActor` Pawn)
    (break)))

(event `self.K2_PostLogin`
  (params (NewPlayer :type "PlayerController Object Reference"))
  ;[1 1 1] ログイン後のHUD作成 ※Delayを挟むのはログイン直後にPlayerCharacterが存在しないことがあるため。
  (if (`Controller.IsLocalPlayerController` NewPlayer)
    (`KismetSystemLibrary.Delay` 0.2)
    (bind _returnvalue (`|CreateWidget` "/Game/P2P/Blueprints/HUDWidget.HUDWidget_C"))
    (`UserWidget.AddToViewport` _returnvalue 0)
    (else
      (bind _asmy_player_controller (cast `` NewPlayer))
      (`self.ClientPostLogin` _asmy_player_controller) ; クライアント側へ送信
    )))

(fn `UserConstructionScript`)