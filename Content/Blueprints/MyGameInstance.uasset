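; Game instance that manages LAN multiplayer sessions and reports network and travel errors.
; Creating a session hosts up to four public connections and opens the battle map as a listen server.
; Finding searches for a single LAN session and joins it, while destroying one returns to the login map.
; Session failures and engine network or travel error types are only printed as strings, with no recovery.
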(event `CreateSession`
  ;[1 1 1] セッションを作成
  (`CreateSessionCallbackProxy.CreateSession` (`GameplayStatics.GetPlayerController` 0) 4 true ; 同時に4人まで
    (:`OnSuccess`
      (`GameplayStatics.OpenLevel` "ExampleBattleMap" true "listen"))
    (:`OnFailure`
      (`KismetSystemLibrary.PrintString` "Create Session Failure" true true (struct :`R` 1.0 :`G` 0.005 :`A` 1.0) 10.0))))

(event `FindSession`
  (bind _returnvalue (`GameplayStatics.GetPlayerController` 0))
  ;[1 1 1] セッションを検索とそのジョイン
  (bind _results (`FindSessionsCallbackProxy.FindSessions` _returnvalue 1 true)
    (:`OnSuccess`
      (for _array_element _results
        (`JoinSessionCallbackProxy.JoinSession` _returnvalue _array_element)))
    (:`OnFailure`
      (`KismetSystemLibrary.PrintString` "Find Session Failure" true true (struct :`R` 1.0 :`G` 0.005 :`A` 1.0) 10.0))))

(event `DestroySession`
  (params (PlayerController :type "PlayerController Object Reference"))
  ;[1 1 1] セッションの破棄
  (`DestroySessionCallbackProxy.DestroySession` PlayerController
    (:`OnSuccess`
      (`GameplayStatics.OpenLevel` "LoginMap"))
    (:`OnFailure`
      (`KismetSystemLibrary.PrintString` "Destroy Session Failure" true true (struct :`R` 1.0 :`G` 0.005 :`A` 1.0) 10.0))))

(event `self.HandleNetworkError`
  (params (FailureType :type "ENetworkFailure Enum" :default "NetDriverAlreadyExists") (bIsServer :type Boolean))
  ;[1 1 1] ネットワークエラーハンドリング
  (switch `ENetworkFailure` FailureType
    (:`NetDriverAlreadyExists`
      _)
    (:`NetDriverCreateFailure`
      _)
    (:`NetDriverListenFailure`
      _)
    (:`ConnectionLost`
      _)
    (:`ConnectionTimeout`
      _)
    (:`FailureReceived`
      _)
    (:`OutdatedClient`
      _)
    (:`OutdatedServer`
      _)
    (:`PendingConnectionFailure`
      _))
  (`KismetSystemLibrary.PrintString` (`KismetStringLibrary.Conv_ByteToString` FailureType) true true (struct :`R` 1.0 :`A` 1.0) 10.0))

(event `self.HandleTravelError`
  (params (FailureType :type "ETravelFailure Enum" :default "NoLevel"))
  ;[1 1 1] トラベルエラーハンドリング
  (switch `ETravelFailure` FailureType
    (:`NoLevel`
      _)
    (:`LoadMapFailure`
      _)
    (:`InvalidURL`
      _)
    (:`PackageMissing`
      _)
    (:`PackageVersion`
      _)
    (:`NoDownload`
      _)
    (:`TravelFailure`
      _)
    (:`CheatCommands`
      _)
    (:`PendingNetGameCreateFailure`
      _)
    (:`CloudSaveFailure`
      _)
    (:`ServerTravelFailure`
      _)
    (:`ClientTravelFailure`
      _))
  (`KismetSystemLibrary.PrintString` (`|GetEnumeratorNameAsString` FailureType) true true (struct :`R` 1.0 :`A` 1.0) 10.0))