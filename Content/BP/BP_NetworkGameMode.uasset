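; Network game mode Blueprint that tracks the NetworkPlayerController of each player in the session.
; It adds controllers to a PlayerControllers array on login, removes them on logout, and swaps old for new when seamless travel replaces them.
; ReadyToStartMatch and ReadyToEndMatch always return false, so the match never starts or ends automatically.
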(event `self.K2_PostLogin`
  (params (NewPlayer :type "PlayerController Object Reference"))
  ;[1 1 1] セッションに参加した
  (bind _asnetwork_player_controller (cast `NetworkPlayerController` NewPlayer))
  (`KismetArrayLibrary.Array_Add` (`self.PlayerControllers`) _asnetwork_player_controller))

(event `self.K2_OnSwapPlayerControllers`
  (params (OldPC :type "PlayerController Object Reference") (NewPC :type "PlayerController Object Reference"))
  (bind (_asnetwork_player_controller _bsuccess) (cast `NetworkPlayerController` NewPC :!pure true))
  (bind (_asnetwork_player_controller_2 _bsuccess_2) (cast `NetworkPlayerController` OldPC :!pure true))
  ;[1 1 1] SeamlessTravelでレベルを移動した時の処理
  (if (and _bsuccess_2 _bsuccess)
    (`KismetArrayLibrary.Array_RemoveItem` (`self.PlayerControllers`) _asnetwork_player_controller_2)
    (`KismetArrayLibrary.Array_Add` (`self.PlayerControllers`) _asnetwork_player_controller)))

(event `self.K2_OnLogout`
  (params (ExitingController :type "Controller Object Reference"))
  ;[1 1 1] プレイヤーがセッションを離脱した時の処理
  (bind _asnetwork_player_controller (cast `NetworkPlayerController` ExitingController))
  (`KismetArrayLibrary.Array_RemoveItem` (`self.PlayerControllers`) _asnetwork_player_controller))

(fn `ReadyToEndMatch`
  (returns (ReturnValue :type Boolean))
  (return false))

(fn `ReadyToStartMatch`
  (returns (ReturnValue :type Boolean))
  (return false))

(fn `UserConstructionScript`)