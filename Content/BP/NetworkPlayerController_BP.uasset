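; Networked player controller that shows a waiting widget after login and drives periodic transform synchronization between client and server.
; ClientPostLogin creates the NetWorkWating widget and adds it to the viewport after a short delay.
; Tick branches on IsServer and uses Delay with GetSynchronousInterval to throttle the RPCs: the server side applies transforms, while the client side transfers them.
; The RPC events only forward to ServerApplyTransform and ClientTransformTransfer, whose logic lives outside these graphs.
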(event `ClientPostLogin`
  (params (NewParam :type Boolean))
  ;[1 1 1] HUD作成
  (`KismetSystemLibrary.Delay` 0.2)
  (bind _returnvalue (`|CreateWidget` "/Game/UI/NetWork/NetWorkWating.NetWorkWating_C" self))
  (`UserWidget.AddToViewport` _returnvalue 0))

(event `self.ReceiveTick`
  (params (DeltaSeconds :type "Float (single-precision)"))
  (bind _returnvalue (`self.GetSynchronousInterval`))
  (if (`KismetSystemLibrary.IsServer`)
    (`KismetSystemLibrary.Delay` _returnvalue)
    (`self.RunOnServer_ApplyTransform`)
    (else
      (`KismetSystemLibrary.Delay` _returnvalue)
      (`self.RunOnOwningClient_TransformTransfer`))))

(event `RunOnOwningClient_TransformTransfer`
  ;[1 1 1] 座標の受け渡しRPC
  (`self.Client_TransformTransfer`))

(event `RunOnServer_ApplyTransform`
  ;[1 1 1] 座標の受け渡しRPC
  (`self.Server_ApplyTransform`))

(fn `UserConstructionScript`)