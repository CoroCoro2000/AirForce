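; Player-controlled drone that drives its motor sound from flight input and carries experimental multiplayer sync events.
; Tick ramps a sound-mix volume through an ExpoIn ease while any stick is active, lowers it when idle, and mutes it once GameManagerBP reports the goal.
; RepLocation and RepRotation apply drone transforms, but the remote-client call feeding them is disconnected.
; Multicast nudges other drones' rotation and its own position, resembling test code.
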(event `Multicast`
  (bind _outactors (`GameplayStatics.GetAllActorsOfClass` "PlayerDrone_BP_C"))
  (for _array_element _outactors
    (if (!= _array_element self)
      (`self.K2_AddActorWorldRotation` _array_element (struct :`Yaw` 1.0) false false)
      (`self.K2_AddActorWorldOffset` (0.0 0.0 0.05))
      (`self.ForceNetUpdate` _array_element))))

(event `self.ReceiveBeginPlay`
  (`GameplayStatics.PushSoundMixModifier` "/Game/Sound/SE/Drone_SeMix.Drone_SeMix")
  (`GameplayStatics.PlaySound2D` "/Game/Sound/SE/Drone_mini_fix_Cue.Drone_mini_fix_Cue" 0.25 1.0 0.0 null null)
  (bind _outactors (`GameplayStatics.GetAllActorsOfClass` "/Game/BP/GameManagerBP.GameManagerBP_C"))
  (for _array_element _outactors
    _)
  (set `self.GameManager` _array_element))

(event `self.ReceiveTick`
  (params (DeltaSeconds :type "Float (single-precision)"))
  (`|ExecutionSequence`
    (:`then_0`
      (if (`GameManager.GetIsGoal` (`self.GameManager`))
        (`/Engine/EditorBlueprintResources/StandardMacros.DoOnce` false
          (:`Completed`
            (`GameplayStatics.SetSoundMixClassOverride` "/Game/Sound/SE/Drone_SeMix.Drone_SeMix" "/Game/Sound/SE/Sound_Drone_Class.Sound_Drone_Class" 0.0)
            (`GameplayStatics.PushSoundMixModifier` "/Game/Sound/SE/Drone_SeMix.Drone_SeMix")))
        (elif (or (> (`self.GetInputValue` "THROTTLE") 0.0) (!= (`self.GetInputValue` "ELEVATOR") 0.0) (!= (`self.GetInputValue` "AILERON") 0.0) (!= (`self.GetInputValue` "LADDER") 0.0))
          (if (<= (`self.Volume`) 1.0)
            (set `self.Volume` (+ (`self.Volume`) 0.05))
            (`GameplayStatics.SetSoundMixClassOverride` "/Game/Sound/SE/Drone_SeMix.Drone_SeMix" "/Game/Sound/SE/Sound_Drone_Class.Sound_Drone_Class" (`|EaseFunction` "ExpoIn" (`self.Volume`) (`self.MinVolume`) (`self.MaxVolume`)) :!label _label))
          (elif (> (`self.Volume`) 0.1)
            (set `self.Volume` (- (`self.Volume`) 0.1))
            (goto _label)))))
    (:`then_1`
      (if (`self.GetisReplay`)
        (set `self.DeltaTime` DeltaSeconds)))))

(event `GetClientDrone`
  ;[1 1 1] 各クライアントのドローン情報をサーバーに送信
  (`self.RepLocation` (`self.GetDroneLocation`))
  (`self.RepRotation` (`self.GetBodyMeshRotation`)))

(event `RepLocation`
  (params (NewParam :type "Vector Structure"))
  ;[1 1 1] サーバーから各ドローン情報を反映
  (`self.K2_SetActorLocation` NewParam))

(event `RepRotation`
  (params (NewParam :type "Rotator Structure"))
  ;[1 1 1] サーバーから各ドローン情報を反映
  (`self.SetBodyMeshRotation` NewParam))

(event `RunOnServer`
  (`KismetSystemLibrary.PrintString` "RunOnServer"))

(fn `UserConstructionScript`)