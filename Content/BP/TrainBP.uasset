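; Train actor that honks a horn when an actor tagged Drone hits it or enters its Carhorn_Collision volume.
; Both the Hit and overlap events play the Carhorn sound at the train's location with boosted volume.
; A shared CanPlaySound flag and a separate DoOnce per event enforce a short cooldown, reset after a delay, to prevent repeated honking.
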(event `self.ReceiveHit`
  (params (MyComp :type "PrimitiveComponent Object Reference") (Other :type "Actor Object Reference") (OtherComp :type "PrimitiveComponent Object Reference") (bSelfMoved :type Boolean) (HitLocation :type "Vector Structure") (HitNormal :type "Vector Structure") (NormalImpulse :type "Vector Structure") (Hit :type "HitResult Structure (by ref)"))
  (if (and (`self.ActorHasTag` Other "Drone") (`self.bCanPlaySound`))
    (`/Engine/EditorBlueprintResources/StandardMacros.DoOnce` false :!label _label
      (:`Completed`
        (`GameplayStatics.PlaySoundAtLocation` "/Game/Sound/SE/carhorn.carhorn" (`self.K2_GetActorLocation`) (struct) 2.5 1.0 0.0 null null null)
        (set `self.bCanPlaySound` false)
        (`KismetSystemLibrary.Delay` 1.0)
        (set `self.bCanPlaySound` true)
        (goto _label :!via `Reset`)))))

(event `self.Carhorn_Collision.OnComponentBeginOverlap`
  (params (OverlappedComponent :type "PrimitiveComponent Object Reference") (OtherActor :type "Actor Object Reference") (OtherComp :type "PrimitiveComponent Object Reference") (OtherBodyIndex :type Integer) (bFromSweep :type Boolean) (SweepResult :type "HitResult Structure (by ref)"))
  (if (and (`self.ActorHasTag` OtherActor "Drone") (`self.bCanPlaySound`))
    (`/Engine/EditorBlueprintResources/StandardMacros.DoOnce` false :!label _label_2
      (:`Completed`
        (`GameplayStatics.PlaySoundAtLocation` "/Game/Sound/SE/carhorn.carhorn" (`self.K2_GetActorLocation`) (struct) 2.5 1.0 0.0 null null null)
        (set `self.bCanPlaySound` false)
        (`KismetSystemLibrary.Delay` 1.0)
        (set `self.bCanPlaySound` true)
        (goto _label_2 :!via `Reset`)))))

(fn `UserConstructionScript`)